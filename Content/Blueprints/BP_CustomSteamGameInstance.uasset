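; Game instance that hosts and joins Steam multiplayer sessions through Advanced Sessions nodes.
; CreateSession tags the session with a GAMENAME property and opens ThirdPersonMap as a listen server on success.
; FindSession filters on that same tag and joins the first result, printing debug messages along the way.
; Both events call OnSearch with a boolean to signal when an operation is in progress, though not every outcome clears it.
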(event `CreateSession`
  (`CreateSessionCallbackProxyAdvanced.CreateAdvancedSession` (`|MakeArray` (`AdvancedSessionsLibrary.MakeLiteralSessionPropertyString` "GAMENAME" "SteamSetup")) (`GameplayStatics.GetPlayerController` 0)
    (:`then`
      (`self.OnSearch` true))
    (:`OnSuccess`
      (`self.OnSearch` false)
      (`GameplayStatics.OpenLevelBySoftObjectPtr` "/Game/Maps/ThirdPersonMap.ThirdPersonMap" true "listen"))))

(event `FindSession`
  (`self.OnSearch` true)
  (bind _results (`FindSessionsCallbackProxyAdvanced.FindSessionsAdvanced` (`GameplayStatics.GetPlayerController` 0) 2147483647 false "AllServers" (`|MakeArray` (`AdvancedSessionsLibrary.MakeLiteralSessionSearchProperty` (`AdvancedSessionsLibrary.MakeLiteralSessionPropertyString` "GAMENAME" "SteamSetup") "Equals")))
    (:`OnSuccess`
      (`self.OnSearch` false)
      (if (`KismetArrayLibrary.Array_IsNotEmpty` _results)
        (`KismetSystemLibrary.PrintString` "Find one !")
        (bind _output (`|GetArrayItem` _results))
        (bind _extrasettings (`AdvancedSessionsLibrary.GetExtraSettings` _output))
        (bind _settingvalue (`AdvancedSessionsLibrary.GetSessionPropertyString` _extrasettings "GAMENAME")
          (:`Found`
            (`KismetSystemLibrary.PrintString` _settingvalue)
            (`JoinSessionCallbackProxy.JoinSession` (`GameplayStatics.GetPlayerController` 0) _output
              (:`OnSuccess`
                (`KismetSystemLibrary.PrintString` "Join Success"))
              (:`OnFailure`
                (`KismetSystemLibrary.PrintString` "Fail Join")
                (`self.OnSearch` false)))))
        (else
          (`KismetSystemLibrary.PrintString` "No Session found")
          (`self.OnSearch` false :!label _label))))
    (:`OnFailure`
      (`KismetSystemLibrary.PrintString` "Fail Find")
      (goto _label))))