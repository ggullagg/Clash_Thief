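; BP_TrapMain is a trap actor, likely a base, that serves as either a local pre-spawn version or a spawned trap.
; Shortly after BeginPlay, a Local instance stops replicating, hides and applies M_BeforeSpawn, while others play an explosion effect at their location.
; SetMaterials swaps every static mesh slot, caching originals in MainMaterials for restoration.
; The cache is keyed by component, so it holds one material per mesh.
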(event `self.ReceiveBeginPlay`
  (`KismetSystemLibrary.Delay` 0.1)
  (if (`self.Local?`)
    (`self.SetReplicates` false)
    (`self.SetActorHiddenInGame` true)
    (`self.SetMaterials` true)
    (else
      (`NiagaraFunctionLibrary.SpawnSystemAtLocation` "/Niagara/DefaultAssets/Templates/Systems/SimpleExplosion.SimpleExplosion" (`self.K2_GetActorLocation`)))))

(fn `SetMaterials`
  (params (`BeforeSpawn?` :type Boolean))
  (for _array_element (`self.K2_GetComponentsByClass` "/Script/Engine.StaticMeshComponent")
    (for _index (range (+ (`KismetArrayLibrary.Array_LastIndex` (`MeshComponent.GetMaterials` _array_element)) 1))
      (if `BeforeSpawn?`
        (`BlueprintMapLibrary.Map_Add` (`self.MainMaterials`) _array_element (`PrimitiveComponent.GetMaterial` _array_element _index)))
      (`PrimitiveComponent.SetMaterial` _array_element _index (select `bool` `BeforeSpawn?` :`false` (`BlueprintMapLibrary.Map_Find` (`self.MainMaterials`) _array_element) :`true` "/Game/Core/AI/M_BeforeSpawn.M_BeforeSpawn")))))

(fn `UserConstructionScript`)