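; Game mode, apparently for the menu, that reports players joining and leaving to the GS_Main game state.
; It caches the cast game state on BeginPlay, then passes each player's PlayerState on from the post-login and logout events.
; Server-named join and leave events forward to GS_Main, and only the login path checks that the cached reference is valid.
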(event `self.ReceiveBeginPlay`
  (bind _asgs_main (cast `/Game/Core/Multiplayer/GS_Main` (`GameplayStatics.GetGameState`)))
  (set `self.GameStateMain` _asgs_main))

(event `self.K2_PostLogin`
  (params (NewPlayer :type "PlayerController Object Reference"))
  (`/Engine/EditorBlueprintResources/StandardMacros.IsValid` (`self.GameStateMain`)
    (:`Is Valid`
      (`self.Server_Player Joined` (`Controller.PlayerState` NewPlayer)))))

(event `self.K2_OnLogout`
  (params (ExitingController :type "Controller Object Reference"))
  (`self.Server_Player leaved` (`Controller.PlayerState` ExitingController)))

(event `Server_Player leaved`
  (params (`New player` :type "PlayerState Object Reference (by ref)"))
  (`/Game/Core/Multiplayer/GS_Main.Server_Player Leaved` (`self.GameStateMain`) `New player`))

(event `Server_Player Joined`
  (params (`New player` :type "PlayerState Object Reference (by ref)"))
  (`/Game/Core/Multiplayer/GS_Main.Server_Player Joined` (`self.GameStateMain`) `New player`))

(fn `UserConstructionScript`)