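; Game instance for Clash_Thief that manages Steam sessions: two-connection hosting, matchmaking, invites, teardown and server travel to GameMap.
; FindSession filters by game name and CanFind, then joins the first result while SearchServer is set.
; Without results it creates a session if none exists, reopening MainMenu as a listen server, and keeps searching while SearchServer stays set.
; Accepting an invite destroys any created session before joining the inviter's.
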(event `self.OnSessionInviteAccepted`
  (params (LocalPlayerNum :type Integer) (PersonInvited :type "BPUniqueNetId Structure") (SessionToJoin :type "BlueprintSessionResult Structure (by ref)"))
  (if (`self.CreatedSession`)
    (`DestroySessionCallbackProxy.DestroySession` (`GameplayStatics.GetPlayerController` 0)
      (:`OnSuccess`
        _)
      (:`OnFailure`
        _)))
  (set `self.SearchServer` false)
  (set `self.CreatedSession` false)
  (`JoinSessionCallbackProxy.JoinSession` (`GameplayStatics.GetPlayerController` 0) SessionToJoin
    (:`OnSuccess`
      (`self.SessionCreated?` false))))

(event `SessionCreated?`
  (params (CreatedSession :type Boolean))
  (set `self.CreatedSession` CreatedSession))

(event `OpenGame`
  (`self.Server_OpenGame`))

(event `CreateSession`
  (if (`self.CreatedSession`)
    (`DestroySessionCallbackProxy.DestroySession` (`GameplayStatics.GetPlayerController` 0)
      (:`OnSuccess`
        _)))
  (`KismetSystemLibrary.PrintString` "creating server")
  (`CreateSessionCallbackProxyAdvanced.CreateAdvancedSession` (`|MakeArray` (`AdvancedSessionsLibrary.MakeLiteralSessionPropertyString` "GameName" "Clash_Thief")) (`GameplayStatics.GetPlayerController` 0) 2
    (:`then`
      (`self.OnSearch` true)
      (`self.SessionCreated?` true))
    (:`OnSuccess`
      (`self.OnSearch` false)
      (`GameplayStatics.OpenLevelBySoftObjectPtr` "/Game/Core/Maps/MainMenu.MainMenu" true "listen"))))

(event `Server_OpenGame`
  (`AdvancedSessionsLibrary.ServerTravel` "GameMap"))

(event `OpenMainMenu`
  (`DestroySessionCallbackProxy.DestroySession` (`GameplayStatics.GetPlayerController` 0)
    (:`OnSuccess`
      (set `self.CreatedSession` false))))

(event `FindSession`
  (`self.OnSearch` true)
  (bind _results (`FindSessionsCallbackProxyAdvanced.FindSessionsAdvanced` (`GameplayStatics.GetPlayerController` 0) 2147483647 false "AllServers" (`|MakeArray` (`AdvancedSessionsLibrary.MakeLiteralSessionSearchProperty` (`AdvancedSessionsLibrary.MakeLiteralSessionPropertyString` "GameName" "Clash_Thief") "Equals") (`AdvancedSessionsLibrary.MakeLiteralSessionSearchProperty` (`AdvancedSessionsLibrary.MakeLiteralSessionPropertyInt` "CanFind" 2) "Equals")))
    (:`OnSuccess`
      (`self.OnSearch` false)
      (if (`KismetArrayLibrary.Array_IsNotEmpty` _results)
        (bind _output (`|GetArrayItem` _results))
        (bind _extrasettings (`AdvancedSessionsLibrary.GetExtraSettings` _output))
        (`AdvancedSessionsLibrary.GetSessionPropertyString` _extrasettings "GameName"
          (:`Found`
            (if (`self.SearchServer`)
              (`JoinSessionCallbackProxy.JoinSession` (`GameplayStatics.GetPlayerController` 0) _output
                (:`OnSuccess`
                  (`self.SessionCreated?` false))
                (:`OnFailure`
                  (`|ExecutionSequence`
                    (:`then_0`
                      (`self.OnSearch` false))
                    (:`then_1`
                      (if (`self.SearchServer`) :!label _label
                        (`self.FindSession`)
                        (else
                          (`self.DestroyServer`))))))))))
        (else
          (`self.OnSearch` false :!label _label_2)
          (if (not (`self.CreatedSession`))
            (`self.CreateSession`)
            (goto _label)))))
    (:`OnFailure`
      (goto _label_2))))

(event `DestroyServer`
  (`DestroySessionCallbackProxy.DestroySession` (`GameplayStatics.GetPlayerController` 0)))

(event `ShowInvite Ui`
  (params (PlayerController :type "PlayerController Object Reference (by ref)"))
  (`AdvancedExternalUILibrary.ShowInviteUI` PlayerController))